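; GM_BPNodes is a game mode Blueprint that demonstrates a set of Blueprint nodes for reading and editing text assets.
; On BeginPlay, a Sequence exercises each operation on TXT_ assets: read, set, append with timestamps, edit lines, export, import and search, printing some results.
; The exported string from one asset feeds the import into another.
; Overview_AllNodes holds an unwired copy of each node as a visual reference.
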(event EventBeginPlay
  (bind _returnvalue (Utilities|Text|MakeLiteralText "Replace line 2 with this text"))
  (Utilities|FlowControl|Sequence
    (:then_0
      (Development|PrintText (Class|TextAssetUEBP|GetText "/Game/TXT_Credits.TXT_Credits")))
    (:then_1
      (Class|TextAssetUEBP|SetText "/Game/TXT_FromBP.TXT_FromBP" (Utilities|Text|MakeLiteralText "This text was created by Blueprint and save at TXT_FromBP")))
    (:then_2
      (Class|TextAssetUEBP|AppendText "/Game/TXT_FromBPAppend.TXT_FromBPAppend" (Utilities|Text|MakeLiteralText "New line with timestamp, a la Output Log") true))
    (:then_3
      (bind _returnvalue_2 (Class|TextAssetUEBP|GetLineCount "/Game/TXT_Credits.TXT_Credits"))
      (Development|PrintString (Utilities|String|Append "TXT_Credits line count: " (Utilities|String|ToString(Integer) _returnvalue_2))))
    (:then_4
      (bind (_outline _returnvalue_3) (Class|TextAssetUEBP|GetLine "/Game/TXT_FromBPAppend.TXT_FromBPAppend" 2))
      (if _returnvalue_3
        (Development|PrintText _outline)))
    (:then_5
      (bind _returnvalue_4 (Class|TextAssetUEBP|RemoveLine "/Game/TXT_FromBPSample.TXT_FromBPSample" 2))
      (if _returnvalue_4
        (Development|PrintText "Line 2 removed from TXT_FromBPSample")))
    (:then_6
      (bind _returnvalue_5 (Class|TextAssetUEBP|ReplaceLine 0 2 _returnvalue))
      (if _returnvalue_5
        (Development|PrintText _returnvalue)))
    (:then_7
      (Class|TextAssetUEBP|AppendLines "/Game/TXT_FromBPAppend.TXT_FromBPAppend" (Utilities|Array|MakeArray "Line1" "Line2" "Line3" "Line4" "Line5") true))
    (:then_8
      (bind _outstring (Class|TextAssetUEBP|ExporttoString "/Game/TXT_FromBPAppend.TXT_FromBPAppend"))
      (Development|PrintString (Utilities|String|Append "TXT_FromBPAppend, Export to String :" _outstring)))
    (:then_9
      (Class|TextAssetUEBP|ImportfromString "/Game/TXT_FromBPImport.TXT_FromBPImport" (Utilities|String|Append "TXT_FromBPAppend, Export to String :" _outstring)))
    (:then_10
      (bind _outlineindices (Class|TextAssetUEBP|FindLinesContaining "/Game/TXT_Credits.TXT_Credits" "orig"))
      (Development|PrintString (Utilities|String|Append "Found lines with \"orig\" at TXT_Credits : " (Utilities|String|ToString(Integer) (Utilities|Array|Length _outlineindices)))))))

(fn ConstructionScript)